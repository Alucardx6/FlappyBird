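; Block is a scrolling Actor that carries a collectible Bean, which awards a point when overlapped.
; On BeginPlay it shifts its root by a random vertical offset, then each Tick moves it along negative X at a constant, frame-rate-independent speed.
; Any overlap with the Bean calls AddPoint on Bp_GameMod, destroys the Bean component and plays the Bite sound.
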(event OnComponentBeginOverlap(Bean)
  (params (OverlappedComponent :type Primitive%20Component%20Object%20Reference) (OtherActor :type Actor%20Object%20Reference) (OtherComp :type Primitive%20Component%20Object%20Reference) (OtherBodyIndex :type Integer) (bFromSweep :type Boolean) (SweepResult :type Hit%20Result%20Structure%20%28by%20ref%29))
  ;[1 1 1] Add Point
  (bind _asbp_game_mod (Utilities|Casting|CastToBp_GameMod (Game|GetGameMode)))
  (Default|AddPoint _asbp_game_mod)
  ;[1 1 1] Kill Bean
  (Components|DestroyComponent (Variables|Default|GetBean))
  (Audio|PlaySound2D "/Game/Sounds/Bite.Bite" 1.0 1.0 0.0 0 0))

(event EventBeginPlay
  (Transformation|SetWorldLocation (Variables|Default|GetDefaultSceneRoot) (+ (Transformation|GetWorldLocation (Variables|Default|GetDefaultSceneRoot)) (Math|Vector|MakeVector 0.0 0.0 (Math|Random|RandomFloatinRange -9e+01 9e+01))) false false))

(event Collision|EventActorBeginOverlap
  (params (OtherActor :type Actor%20Object%20Reference)))

(event EventTick
  (params (DeltaSeconds :type Float%20%28single-precision%29))
  (Transformation|SetWorldLocation (Variables|Default|GetDefaultSceneRoot) (+ (Transformation|GetWorldLocation (Variables|Default|GetDefaultSceneRoot)) (Math|Vector|MakeVector (* DeltaSeconds (Math|Float|MakeLiteralFloat -1e+02)) 0.0 0.0)) false false))

(fn ConstructionScript)